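; Spawner that keeps up to MaxSpawnItem Gold actors placed at random spawn points.
; Tick tops up the count via ItemSpawn, which retries random GoldSpawnPoint slots until one is free, though check, spawn and marking each roll separate indices.
; Tick also binds each item's OnDestroyed to DestroyedEvent, which decrements the count and frees the slot at the last stored ArrayIndex, not necessarily the destroyed item's.
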(event Custom|DestroyedEvent
  (params (DestroyedActor :type Actor%20Object%20Reference))
  (Math|Integer|DecrementInt (Variables|Default|GetSpawnItem)
    (:%20%20
      (|SetBy-RefVar (Utilities|Array|Get(acopy) (Variables|Default|GetGoldSpawnPoint) (Variables|Default|GetArray%20Index))))))

(event EventBeginPlay
  (Variables|Default|SetSpawnItem 0))

(event Collision|EventActorBeginOverlap
  (params (OtherActor :type Actor%20Object%20Reference)))

(event EventTick
  (params (DeltaSeconds :type Float%20%28single-precision%29))
  (Utilities|FlowControl|Sequence
    (:then_0
      (if (< (Variables|Default|GetSpawnItem) (Variables|Default|GetMaxSpawnItem))
        (for _index (range 0 (- (Variables|Default|GetMaxSpawnItem) (Variables|Default|GetSpawnItem)))
          (Variables|Default|SetEndSpawn false)
          (CallFunction|ItemSpawn)
          (Math|Integer|IncrementInt (Variables|Default|GetSpawnItem)))))
    (:then_1
      (if (> (Variables|Default|GetSpawnItem) 0)
        (for (_array_element _array_index) (Variables|Default|GetGoldSpawnPoint)
          (Variables|Default|SetArray%20Index _array_index)
          (if (Utilities|IsValid (.Item (Utilities|Struct|BreakGoldData _array_element)))
            (Game|AssignOnDestroyed (.Item (Utilities|Struct|BreakGoldData _array_element)) (delegate Custom|DestroyedEvent))))))))

(fn ConstructionScript)

(fn ItemSpawn
  (bind _spawnpoint (Variables|Default|GetSpawnPoint))
  (bind _returnvalue (Utilities|Array|Length _spawnpoint))
  (bind _returnvalue_2 (Math|Random|RandomInteger _returnvalue))
  (while (not (Variables|Default|GetEndSpawn))
    (if (.canspawn (Utilities|Array|Get(acopy) (Variables|Default|GetGoldSpawnPoint) _returnvalue_2))
      (bind _returnvalue_3 (Game|SpawnActorfromClass "/Game/member/toyama/BP/Gold.Gold_C" (Transformation|GetActorTransform (Utilities|Array|Get(acopy) (Variables|Default|GetSpawnPoint) _returnvalue_2)) "Undefined" 0 0))
      (|SetBy-RefVar (Utilities|Array|Get(acopy) (Variables|Default|GetGoldSpawnPoint) _returnvalue_2) (Utilities|Struct|MakeGoldData false _returnvalue_3))
      (Variables|Default|SetEndSpawn true))))